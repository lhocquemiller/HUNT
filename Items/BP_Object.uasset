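; BP_Object is an item Blueprint that holds a name and flags for whether the item is consumable or equipable.
; Simple setter and getter functions expose the Name, Consumable and Equipable variables.
; The event graph is empty apart from disabled BeginPlay and Tick stubs, so the asset has no behavior of its own.
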(event EventBeginPlay)

(event EventTick
  (params (DeltaSeconds :type Float%20%28single-precision%29)))

(fn SetConsumable
  (params (NewValue :type Boolean))
  (Variables|Default|SetConsumable NewValue))

(fn SetEquipable
  (params (NewValue :type Boolean))
  (Variables|Default|SetEquipable NewValue))

(fn IsConsumable
  (return (Variables|Default|GetConsumable)))

(fn IsEquipable
  (return (Variables|Default|GetEquipable)))

(fn SetName
  (params (Value :type Text))
  (Variables|Default|SetName Value))

(fn GetName
  (return (Variables|Default|GetName)))