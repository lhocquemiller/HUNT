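; BP_Consumable is a usable item with effect, strength, quantity, cooldown and icon, currently supporting an instant health potion scaled by level.
; Consume marks the hero's slot unready, then, unless the item is a mock, applies the effect.
; A successful effect decrements quantity and passes the cooldown to the hero's counter.
; EndOfCooldown re-readies the slot and clears it when quantity reaches zero.
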(event EventBeginPlay
  (CallFunction|SetRoundIcon "/Game/Hunt/Items/Icons/Empty80pixelSquareIcon.Empty80pixelSquareIcon"))

(fn GetCooldown
  (return (Variables|Default|GetCooldown)))

(fn SetEquippedasConsumable
  (params (Value :type Boolean))
  (Variables|Default|SetEquippedAsConsumable Value))

(fn SetMock
  (params (Value :type Boolean))
  (bind _output_get (Variables|Default|SetMock Value))
  (if _output_get
    _))

(fn IsMock
  (return (Variables|Default|GetMock)))

(fn GetRoundIcon
  (return (Variables|Default|GetRoundIcon)))

(fn SetRoundIcon
  (params (Texture :type Texture%202D%20Object%20Reference))
  (Variables|Default|SetRoundIcon Texture))

(fn SetCooldown
  (params (NewCooldown :type Float%20%28single-precision%29))
  (Variables|Default|SetCooldown NewCooldown))

(fn CreateHealthPotion
  (params (Level :type Float%20%28single-precision%29) (Number :type Integer))
  (CallFunction|SetCooldown 5.0)
  (CallFunction|SetName "Health Potion")
  (CallFunction|SetEffect "NewEnumerator0")
  (CallFunction|SetStrength (* 20 (+ Level 1.0)))
  (CallFunction|SetRoundIcon "/Game/Hunt/Items/RoundConsumableIcons/PotionVerte.PotionVerte")
  (CallFunction|SetQuantity Number))

(fn ApplyEffect
  (params (Hero :type BP%20Heroe%20Object%20Reference))
  (switch Utilities|FlowControl|Switch|SwitchonConsumableEffect (Variables|Default|GetEffect)
    (:NewEnumerator1
      (LocalVariables|SetUsed false))
    (:NewEnumerator0
      (bind _healed (Default|HealFixedValue Hero (Variables|Default|GetStrength)))
      (LocalVariables|SetUsed _healed)))
  (return (LocalVariables|GetUsed)))

(fn SetEffect
  (params (NewValue :type ConsumableEffect%20Enum :default "NewEnumerator0"))
  (Variables|Default|SetEffect NewValue))

(fn SetStrength
  (params (NewValue :type Float%20%28single-precision%29))
  (Variables|Default|SetStrength NewValue))

(fn SetQuantity
  (params (NewValue :type Integer))
  (Variables|Default|SetQuantity NewValue))

(fn GetQuantity
  (return (Variables|Default|GetQuantity)))

(fn Consume
  (params (Hero :type BP%20Heroe%20Object%20Reference) (ConsumableIndex :type Integer))
  (bind _output_get (Variables|Default|SetConsumableIndex ConsumableIndex))
  (bind _output_get_2 (LocalVariables|SetUserRef Hero))
  (bind _value (Default|GetConsumableReady _output_get_2 _output_get))
  (if _value
    (Default|SetConsumableReady (LocalVariables|GetUserRef) _output_get false)
    (bind _value_2 (CallFunction|IsMock self))
    (if (not _value_2)
      (bind _success (CallFunction|ApplyEffect (LocalVariables|GetUserRef)))
      (if _success
        (bind _result (Math|Integer|DecrementInt (Variables|Default|GetQuantity))
          (:%20%20
            (Variables|Default|SetQuantity _result)
            (bind _value_3 (CallFunction|GetCooldown self))
            (Default|SetConsumableCounter (LocalVariables|GetUserRef) (Variables|Default|GetConsumableIndex) _value_3)))))))

(fn EndOfCooldown
  (params (Hero :type BP%20Heroe%20Object%20Reference))
  (bind _consumableindex (Variables|Default|GetConsumableIndex))
  (Default|SetConsumableReady Hero _consumableindex true)
  (bind _quantity (CallFunction|GetQuantity))
  (if (== _quantity 0)
    (Default|CleanConsumableSlot Hero _consumableindex)))