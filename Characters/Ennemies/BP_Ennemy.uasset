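; Base enemy Blueprint that reacts to damage and death, with multicast events for networked play.
; While alive, it forwards damage to multicast and server handlers, then tells its AI_Ennemy controller to engage or retarget using the damage causer.
; At zero health it sets Dead, multicasts the death animation, unpossesses and calls SimulatePhysics, an empty event here.
; Accessors expose appearance, death state and melee, jump and forgiveness radii.
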(event Custom|SimulatePhysics)

(event Game|Damage|EventAnyDamage
  (params (Damage :type Float%20%28single-precision%29) (DamageType :type Damage%20Type%20Object%20Reference) (InstigatedBy :type Controller%20Object%20Reference) (DamageCauser :type Actor%20Object%20Reference))
  (bind _value (CallFunction|IsDead))
  (if (not _value)
    (CallFunction|AnyDamageMulticast Damage)
    (CallFunction|AnyDamagesonServer Damage)
    (bind _asai_ennemy (Utilities|Casting|CastToAI_Ennemy (Pawn|GetController)))
    (bind _isincombat (Default|IsinCombat _asai_ennemy))
    (if _isincombat
      (Default|SetNearestPlayerasTarget _asai_ennemy DamageCauser)
      (else
        (Default|EngageCombatonPlayer _asai_ennemy DamageCauser)))
    (bind _value_2 (CallFunction|GetHealth))
    (if (<= _value_2 0.0)
      (Variables|Default|SetDead true)
      (CallFunction|PlayDeathAnimationMulticast)
      (Pawn|UnPossess (Pawn|GetController))
      (CallFunction|SimulatePhysics))))

(fn ConstructionScript)

(fn GetAppearence
  (return (Variables|Default|GetAppearence)))

(fn SetAppearence
  (params (Value :type Ennemies%20Enum :default "NewEnumerator0"))
  (Variables|Default|SetAppearence Value))

(fn GetDead
  (return (Variables|Default|GetDead)))

(fn SetDead
  (params (Value :type Boolean))
  (Variables|Default|SetDead Value))

(fn GetMeleeAcceptanceRadius
  (return (Variables|Default|GetMeleeAcceptanceRadius)))

(fn GetJumpRadius
  (return (Variables|Default|GetJumpRadius)))

(fn GetForgivenessRadius
  (return (Variables|Default|GetForgivenessRadius)))