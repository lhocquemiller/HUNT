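; Base character for combatants, handling health, melee damage, death and servitor minions, with death animation events meant for child classes to override.
; The melee box damages tagged players or AI, and strong attacks also push victims away.
; Damage updates health and combat text, flags victim and attacker as in combat for a delay, notifying servitor AI, and unpossesses at zero health.
; Server-and-multicast event pairs mirror animation, velocity and rotation.
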(event OnComponentBeginOverlap(MeleeBox)
  (params (OverlappedComponent :type Primitive%20Component%20Object%20Reference) (OtherActor :type Actor%20Object%20Reference) (OtherComp :type Primitive%20Component%20Object%20Reference) (OtherBodyIndex :type Integer) (bFromSweep :type Boolean) (SweepResult :type Hit%20Result%20Structure%20%28by%20ref%29))
  (if (or (Actor|ActorHasTag OtherActor "AI") (Actor|ActorHasTag OtherActor "Player"))
    (if (!= OtherActor self)
      (Game|Damage|ApplyDamage OtherActor (Variables|Default|GetBaseDamages) 0 self "/Script/Engine.DamageType")
      (if (Variables|Default|GetStrongAttack)
        (bind _asbp_character (Utilities|Casting|CastToBP_Character OtherActor))
        (CallFunction|GetPushed _asbp_character self)))))

(event Custom|PlayAnimationMontageMulticast
  (params (AnimationMontage :type Anim%20Montage%20Object%20Reference))
  (Components|Animation|PlayAnimation (Variables|Character|GetMesh) AnimationMontage false))

(event Custom|DisableCollisionOnServer
  ;[1 1 1] TakeDamagesAndDie
  (CallFunction|DisableCollisionMulticast)
  (Collision|SetCollisionEnabled (Variables|Collision|GetCapsuleComponent) "NoCollision"))

(event Custom|SetActorRotationMulticast
  (params (Rotator :type Rotator))
  (Transformation|SetActorRotation Rotator))

(event Custom|SetActorRotationOnServerAndMulticast
  (params (Rotator :type Rotator))
  (CallFunction|SetActorRotationMulticast Rotator)
  (Transformation|SetActorRotation Rotator))

(event Custom|AnyDamagesOnServer
  (params (Damage :type Float%20%28single-precision%29))
  ;[1 1 1] TakeDamagesAndDie
)

(event Custom|PlayAnimationMontageOnServerAndMulticast
  (params (AnimationMontage :type Anim%20Montage%20Object%20Reference))
  (CallFunction|PlayAnimationMontageMulticast AnimationMontage)
  (Components|Animation|PlayAnimation (Variables|Character|GetMesh) AnimationMontage false))

(event Custom|PlayDeathAnimationOnServer
  ;[1 1 1] TakeDamagesAndDie
  (CallFunction|PlayDeathAnimationMulticast)
  (Components|Animation|PlayAnimation (Variables|Character|GetMesh) "/Game/Hunt/Characters/Ennemies/MountainDragon/Animations/ANIM_MOUNTAIN_DRAGON_death.ANIM_MOUNTAIN_DRAGON_death" false))

(event Custom|PlayDeathAnimationMulticast
  ;[1 1 1] TakeDamagesAndDie
  (Components|Animation|PlayAnimation (Variables|Character|GetMesh) "/Game/Hunt/Characters/Ennemies/MountainDragon/Animations/ANIM_MOUNTAIN_DRAGON_death.ANIM_MOUNTAIN_DRAGON_death" false))

(event Custom|PutInCombat
  ;[1 1 1] TakeDamagesAndDie
  (CallFunction|InCombat true)
  (Utilities|FlowControl|Delay 1e+01)
  (CallFunction|InCombat false))

(event Custom|DisableCollisionMulticast
  ;[1 1 1] TakeDamagesAndDie
)

(event Custom|SetVelocityMulticast
  (params (Velocity :type Vector))
  (Variables|/Script/Engine.MovementComponent|SetVelocity (Variables|Character|GetCharacterMovement) Velocity))

(event Custom|SetVelocityOnServerAndMulticast
  (params (Velocity :type Vector))
  (CallFunction|SetVelocityMulticast Velocity)
  (Variables|/Script/Engine.MovementComponent|SetVelocity (Variables|Character|GetCharacterMovement) Velocity))

(event Custom|AnyDamageMulticast
  (params (Damage :type Float%20%28single-precision%29))
  ;[1 1 1] TakeDamagesAndDie
  (Default|PlayCombatText (Variables|Default|GetCombatTextReference) Damage)
  (Variables|Default|SetHealth (- (Variables|Default|GetHealth) Damage)))

(event Custom|JustHitSomething
  ;[1 1 1] TakeDamagesAndDie
  (CallFunction|InCombat true)
  (Utilities|FlowControl|Delay 1e+01)
  (CallFunction|InCombat false))

(event Custom|SetAnimInstanceClassMulticast
  (params (AnimClass :type Object%20Class%20Reference))
  (Class|SkeletalMeshComponent|SetAnimClass (Variables|Character|GetMesh) AnimClass))

(event Custom|SetAnimInstanceClassOnServerAndMulticast
  (params (AnimClass :type Object%20Class%20Reference))
  (CallFunction|SetAnimInstanceClassMulticast AnimClass)
  (Class|SkeletalMeshComponent|SetAnimClass (Variables|Character|GetMesh) AnimClass))

(event Game|Damage|EventAnyDamage
  (params (Damage :type Float%20%28single-precision%29) (DamageType :type Damage%20Type%20Object%20Reference) (InstigatedBy :type Controller%20Object%20Reference) (DamageCauser :type Actor%20Object%20Reference))
  ;[1 1 1] TakeDamagesAndDie
  (bind _dead (CallFunction|GetDead))
  (if (not _dead)
    (CallFunction|AnyDamageMulticast Damage)
    (CallFunction|AnyDamagesonServer Damage)
    (CallFunction|PutinCombat)
    (bind _asbp_character (Utilities|Casting|CastToBP_Character DamageCauser)
      (:then
        (CallFunction|JustHitSomething _asbp_character))
      (:CastFailed
        _))
    (bind _value (CallFunction|GetHealth))
    (if (<= _value 0.0)
      (Variables|Default|SetDead true)
      (Pawn|UnPossess (Pawn|GetController))
      (CallFunction|PlayDeathAnimationMulticast))))

(event EventBeginPlay
  (Variables|Default|SetCombatTextReference (.AsDamage%20Display (Utilities|Casting|CastToDamageDisplay (UserInterface|GetUserWidgetObject (Variables|Default|GetCombatText))))))

(fn ConstructionScript)

(fn SetMovementSpeed
  (params (Value :type Float%20%28single-precision%29))
  (bind _output_get (Variables|Default|SetMovementSpeed Value))
  (Variables|/Script/Engine.CharacterMovementComponent|SetMaxWalkSpeed (Variables|Character|GetCharacterMovement) _output_get))

(fn GetMovementSpeed
  (return (Variables|Default|GetMovementSpeed)))

(fn SetMeleeAttacking
  (params (Value :type Boolean))
  (Variables|Default|SetMeleeAttacking Value))

(fn GetMeleeAttacking
  (return (Variables|Default|GetMeleeAttacking)))

(fn GetFalling
  (return (Variables|Default|GetFalling)))

(fn SetFalling
  (params (Value :type Boolean))
  (Variables|Default|SetFalling Value))

(fn GetHealth
  (return (Variables|Default|GetHealth)))

(fn GetMaxHealth
  (return (Variables|Default|GetMaxHealth)))

(fn SetHealth
  (params (Value :type Float%20%28single-precision%29))
  (Variables|Default|SetHealth Value))

(fn SetMaxHealth
  (params (Value :type Float%20%28single-precision%29))
  (Variables|Default|SetMaxHealth Value))

(fn GetBaseDamages
  (return (Variables|Default|GetBaseDamages)))

(fn SetBaseDamages
  (params (Value :type Float%20%28single-precision%29))
  (Variables|Default|SetBaseDamages Value))

(fn SetAnimationonGoing
  (params (Value :type Boolean))
  (Variables|Default|SetAnimationOnGoing Value))

(fn GetAnimationonGoing
  (return (Variables|Default|GetAnimationOnGoing)))

(fn SetStrongAttack
  (params (Value :type Boolean))
  (Variables|Default|SetStrongAttack Value))

(fn GetStrongAttack
  (return (Variables|Default|GetStrongAttack)))

(fn GetPushed
  (params (Attacker :type BP%20Character%20Object%20Reference))
  (bind _returnvalue (Transformation|GetActorLocation Attacker))
  (bind _self self)
  (bind _returnvalue_2 (Transformation|GetActorLocation _self))
  (bind _returnvalue_3 (Math|Vector|GetUnitDirection(Vector) _returnvalue _returnvalue_2))
  (bind (_x _y _z) (Math|Vector|BreakVector _returnvalue_3))
  (Character|Jump)
  (CallFunction|SetVelocityonServerandMulticast (Math|Vector|MakeVector (* _x (LocalVariables|GetPushMultiplier)) (* _y (LocalVariables|GetPushMultiplier)) _z)))

(fn GetDead
  (return (Variables|Default|GetDead)))

(fn InCombat
  (params (InCombat :type Boolean))
  (Variables|Default|SetIsInCombat InCombat)
  (CallFunction|TellServitorstoEngageCombat))

(fn IsCombat
  (return (Variables|Default|GetIsInCombat)))

(fn AddServitor
  (params (Servitor :type BP%20Servitor%20Object%20Reference))
  (Variables|Default|SetServitorIndex (+ (Variables|Default|GetServitorIndex) 1))
  (Utilities|Array|SetArrayElem (Variables|Default|GetServitors) (Variables|Default|GetServitorIndex) Servitor)
  (return (Variables|Default|GetServitorIndex)))

(fn TellServitorstoEngageCombat
  (for _array_element (Variables|Default|GetServitors)
    (bind _asai_servitor (Utilities|Casting|CastToAI_Servitor (Pawn|GetController _array_element)))
    (Default|MasterEngageCombat _asai_servitor)))

(fn KillAllServitors
  (for _array_element (Variables|Default|GetServitors)
    (CallFunction|PlayDeathAnimationonServer _array_element)))