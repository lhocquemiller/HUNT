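; BP_EquippedConsumables is a hero-side Blueprint that stores the consumables equipped in five separate slot variables.
; SetConsomable takes an index and a consumable, then writes it to the matching slot through a chain of equality branches, ignoring indices outside the five slots.
; The event graph holds only disabled BeginPlay and Tick stubs, so the asset acts purely as a data holder.
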(event EventBeginPlay)

(event EventTick
  (params (DeltaSeconds :type Float%20%28single-precision%29)))

(fn SetConsomable
  (params (Index :type Integer) (NewConsumable :type BP%20Object%20Object%20Reference))
  (if (== Index 0)
    (Variables|Default|SetConsomable1 NewConsumable)
    (elif (== Index 1)
      (Variables|Default|SetConsomable2 NewConsumable)
      (elif (== Index 2)
        (Variables|Default|SetConsomable3 NewConsumable)
        (elif (== Index 3)
          (Variables|Default|SetConsomable4 NewConsumable)
          (elif (== Index 4)
            (Variables|Default|SetConsomable5 NewConsumable)))))))