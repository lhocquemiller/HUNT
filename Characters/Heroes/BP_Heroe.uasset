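; Base hero character for the Warrior, Mage and Hunter classes, handling abilities, consumables, damage, death and respawn.
; On possession it builds the client HUD, fills empty slots with mock placeholders, then equips four class spells.
; Input activates abilities or the wheel-selected consumable, with per-slot Delay events ending cooldowns and Tick counting down their timers.
; Death unpossesses and shows a death screen; respawn goes through HuntGameInstance before destroying the old actor.
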(event Custom|LeftClickAnimation
  (Default|ReticuleAnimation (Variables|Default|GetReticuleReference)))

(event Custom|BeginPlayOnClient)

(event Custom|AbilityRequested
  (params (SpellIndex :type Integer))
  (bind _success (Default|OnSpellActivation (Utilities|Array|Get(acopy) (Variables|Default|GetEquippedAbilities) SpellIndex) self SpellIndex))
  (if _success
    (switch int SpellIndex
      (:0
        (CallFunction|Ability1Delay))
      (:1
        (CallFunction|Ability2Delay))
      (:2
        (CallFunction|Ability3Delay))
      (:3
        (CallFunction|Ability4Delay)))))

(event Custom|ConsumableUp
  ;[1 1 1] ConsumableSelection
  (if (== (Variables|Default|GetSelectedConsumableIndex) 0)
    (Variables|Default|SetSelectedConsumableIndex 4)
    (else
      (bind _result (Math|Integer|DecrementInt (Variables|Default|GetSelectedConsumableIndex))
        (:%20%20
          (Variables|Default|SetSelectedConsumableIndex _result)))))
  (Default|UpdateConsumableWidget (Variables|Default|GetConsumableReference)))

(event Custom|RemoveOldWidgetsOnRespawn
  (Widget|RemovefromParent (Variables|Default|GetHealthBarReference))
  (Widget|RemovefromParent (Variables|Default|GetReticuleReference))
  (Widget|RemovefromParent (Variables|Default|GetDeadScreenReference))
  (Widget|RemovefromParent (Variables|Default|GetAbilityBarReference))
  (Widget|RemovefromParent (Variables|Default|GetConsumableReference)))

(event Custom|ConsumableDown
  ;[1 1 1] ConsumableSelection
  (if (== (Variables|Default|GetSelectedConsumableIndex) 4)
    (Variables|Default|SetSelectedConsumableIndex 0)
    (else
      (bind _result (Math|Integer|IncrementInt (Variables|Default|GetSelectedConsumableIndex))
        (:%20%20
          (Variables|Default|SetSelectedConsumableIndex _result)))))
  (Default|UpdateConsumableWidget (Variables|Default|GetConsumableReference)))

(event Custom|DelayOnConsumable1
  (bind _equippedconsumables (Variables|Default|GetEquippedConsumables))
  (bind _output (Utilities|Array|Get(acopy) _equippedconsumables))
  ;[1 1 1] DelayOnConsumableAndAbilities
  (bind _value (Default|GetCooldown _output))
  (Utilities|FlowControl|Delay _value)
  (Default|EndOfCooldown _output self))

(event Custom|DelayOnConsumable2
  (bind _equippedconsumables (Variables|Default|GetEquippedConsumables))
  (bind _output (Utilities|Array|Get(acopy) _equippedconsumables 1))
  ;[1 1 1] DelayOnConsumableAndAbilities
  (bind _value (Default|GetCooldown _output))
  (Utilities|FlowControl|Delay _value)
  (Default|EndOfCooldown _output self))

(event Custom|Ability4Delay
  (bind _equippedabilities (Variables|Default|GetEquippedAbilities))
  (bind _output (Utilities|Array|Get(acopy) _equippedabilities 3))
  ;[1 1 1] DelayOnConsumableAndAbilities
  (bind _value (Default|GetCooldown _output))
  (Utilities|FlowControl|Delay _value)
  (Default|EndOfCooldown _output self))

(event Custom|RequestRespawn
  (CallFunction|RemoveOldWidgetsonRespawn)
  (Variables|/Script/Engine.PlayerController|SetbShowMouseCursor (Variables|Default|GetPlayerController) false)
  (bind _ashunt_game_instance (Utilities|Casting|CastToHuntGameInstance (Game|GetGameInstance)))
  (Default|RespawnCharacter _ashunt_game_instance self (Variables|Default|GetPlayerController))
  (Utilities|FlowControl|Delay 3e+01)
  (Actor|DestroyActor))

(event Custom|DelayOnConsumable4
  (bind _equippedconsumables (Variables|Default|GetEquippedConsumables))
  (bind _output (Utilities|Array|Get(acopy) _equippedconsumables 3))
  ;[1 1 1] DelayOnConsumableAndAbilities
  (bind _value (Default|GetCooldown _output))
  (Utilities|FlowControl|Delay _value)
  (Default|EndOfCooldown _output self))

(event Custom|DelayOnConsumable3
  (bind _equippedconsumables (Variables|Default|GetEquippedConsumables))
  (bind _output (Utilities|Array|Get(acopy) _equippedconsumables 2))
  ;[1 1 1] DelayOnConsumableAndAbilities
  (bind _value (Default|GetCooldown _output))
  (Utilities|FlowControl|Delay _value)
  (Default|EndOfCooldown _output self))

(event Custom|DelayOnConsumable5
  (bind _equippedconsumables (Variables|Default|GetEquippedConsumables))
  (bind _output (Utilities|Array|Get(acopy) _equippedconsumables 4))
  ;[1 1 1] DelayOnConsumableAndAbilities
  (bind _value (Default|GetCooldown _output))
  (Utilities|FlowControl|Delay _value)
  (Default|EndOfCooldown _output self))

(event Custom|Ability1Delay
  (bind _equippedabilities (Variables|Default|GetEquippedAbilities))
  (bind _output (Utilities|Array|Get(acopy) _equippedabilities))
  ;[1 1 1] DelayOnConsumableAndAbilities
  (bind _value (Default|GetCooldown _output))
  (Utilities|FlowControl|Delay _value)
  (Default|EndOfCooldown _output self))

(event Custom|ShowDeathScreen
  ;[1 1 1] TakeDamagesAndDie
  (UserInterface|Viewport|AddtoViewport (Variables|Default|GetDeadScreenReference) 10)
  (bind _asbp_player_controller (Utilities|Casting|CastToBP_PlayerController (Pawn|GetController)))
  (bind _output_get (Variables|Default|SetPlayerController _asbp_player_controller))
  (Variables|/Script/Engine.PlayerController|SetbShowMouseCursor _output_get true))

(event Custom|Ability2Delay
  (bind _equippedabilities (Variables|Default|GetEquippedAbilities))
  (bind _output (Utilities|Array|Get(acopy) _equippedabilities 1))
  ;[1 1 1] DelayOnConsumableAndAbilities
  (bind _value (Default|GetCooldown _output))
  (Utilities|FlowControl|Delay _value)
  (Default|EndOfCooldown _output self))

(event Custom|Ability3Delay
  (bind _equippedabilities (Variables|Default|GetEquippedAbilities))
  (bind _output (Utilities|Array|Get(acopy) _equippedabilities 2))
  ;[1 1 1] DelayOnConsumableAndAbilities
  (bind _value (Default|GetCooldown _output))
  (Utilities|FlowControl|Delay _value)
  (Default|EndOfCooldown _output self))

(event Custom|PossessedOnClient
  (bind _returnvalue (UserInterface|CreateWidget "/Game/Hunt/Interface/HealthBar/HealthBar.HealthBar_C"))
  (bind _output_get (Variables|Default|SetHealthBarReference _returnvalue))
  (Default|SetHeroe _output_get self)
  (UserInterface|Viewport|AddtoViewport _output_get 0)
  (bind _returnvalue_2 (UserInterface|CreateWidget "/Game/Hunt/Interface/Reticule/CentralReticule.CentralReticule_C"))
  (bind _output_get_2 (Variables|Default|SetReticuleReference _returnvalue_2))
  (UserInterface|Viewport|AddtoViewport _output_get_2 0)
  (bind _returnvalue_3 (UserInterface|CreateWidget "/Game/Hunt/Interface/DeadScreen/DeadScreen.DeadScreen_C"))
  (bind _output_get_3 (Variables|Default|SetDeadScreenReference _returnvalue_3))
  (Default|SetHero _output_get_3 self)
  (bind _returnvalue_4 (Game|AddComponentbyClass "/Game/Hunt/Spells/BP_Spell.BP_Spell_C")) ; Base empty consomable
  (Variables|Default|SetMockSpellReference _returnvalue_4)
  (Default|SetMock _returnvalue_4 true)
  (bind _returnvalue_5 (UserInterface|CreateWidget "/Game/Hunt/Interface/Spells/Spells.Spells_C"))
  (bind _output_get_4 (Variables|Default|SetAbilityBarReference _returnvalue_5))
  (Default|SetHero _output_get_4 self)
  (UserInterface|Viewport|AddtoViewport _output_get_4 0)
  (CallFunction|CleanAbilitySlots)
  (CallFunction|AddSpellsonPossessed (Variables|Default|GetClasse))
  (bind _returnvalue_6 (Game|AddComponentbyClass "/Game/Hunt/Items/BP_Consumable.BP_Consumable_C")) ; Base empty consomable
  (Variables|Default|SetMockConsumableReference _returnvalue_6)
  (Default|SetMock _returnvalue_6 true)
  (bind _returnvalue_7 (UserInterface|CreateWidget "/Game/Hunt/Interface/Consumables/Consumables.Consumables_C"))
  (bind _output_get_5 (Variables|Default|SetConsumableReference _returnvalue_7))
  (Default|SetHero _output_get_5 self)
  (UserInterface|Viewport|AddtoViewport _output_get_5 0)
  (CallFunction|CleanConsumableSlots)
  (for (_ _array_index) (Variables|Default|GetEquippedConsumables)
    (Default|SetCooldown (Variables|Default|GetConsumableReference) _array_index 1.0)))

(event Custom|ConsumableRequested
  (bind _selectedconsumableindex (Variables|Default|GetSelectedConsumableIndex))
  ;[1 1 1] ConsumableSelection
  (Default|Consume (Utilities|Array|Get(acopy) (Variables|Default|GetEquippedConsumables) _selectedconsumableindex) self _selectedconsumableindex)
  (switch int _selectedconsumableindex
    (:0
      (CallFunction|DelayonConsumable1))
    (:1
      (CallFunction|DelayonConsumable2))
    (:2
      (CallFunction|DelayonConsumable3))
    (:3
      (CallFunction|DelayonConsumable4))
    (:4
      (CallFunction|DelayonConsumable5))))

(event Custom|BeginPlayOnAll
  (Variables|Default|SetCombatTextReference (.AsDamage%20Display (Utilities|Casting|CastToDamageDisplay (UserInterface|GetUserWidgetObject (Variables|Default|GetCombatText))))))

(event Game|Damage|EventAnyDamage
  (params (Damage :type Float%20%28single-precision%29) (DamageType :type Damage%20Type%20Object%20Reference) (InstigatedBy :type Controller%20Object%20Reference) (DamageCauser :type Actor%20Object%20Reference))
  ;[1 1 1] TakeDamagesAndDie
  (bind _value (CallFunction|IsDead))
  (if (not _value)
    (CallFunction|AnyDamageMulticast Damage)
    (CallFunction|AnyDamagesonServer Damage)
    (bind _value_2 (CallFunction|GetHealth))
    (if (<= _value_2 0.0)
      (Variables|Default|SetDead true)
      (CallFunction|PlayDeathAnimationMulticast)
      (CallFunction|ShowDeathScreen)
      (Pawn|UnPossess (Pawn|GetController)))))

(event EventBeginPlay
  (CallFunction|BeginPlayonAll)
  (CallFunction|BeginPlayonClient))

(event EventTick
  (params (DeltaSeconds :type Float%20%28single-precision%29))
  ;[1 1 1] OnTick: Update ability and consumable counters
  (for (_array_element _array_index) (Variables|Default|GetAbilityReady)
    (if (not _array_element)
      (bind _counter (CallFunction|GetAbilityCounter _array_index))
      (CallFunction|SetAbilityCounter _array_index (- _counter DeltaSeconds))))
  (for (_array_element_2 _array_index_2) (Variables|Default|GetConsumableReady)
    (if (not _array_element_2)
      (bind _counter_2 (CallFunction|GetConsumableCounter _array_index_2))
      (CallFunction|SetConsumableCounter _array_index_2 (- _counter_2 DeltaSeconds)))))

(event EventPossessed
  (params (NewController :type Controller%20Object%20Reference))
  (CallFunction|PossessedonClient))

(event Input|KeyboardEvents|1
  (params (Key :type Key%20Structure :default "None"))
  ;[1 1 1] Control
)

(event Input|MouseEvents|RightMouseButton
  (params (Key :type Key%20Structure :default "None"))
  ;[1 1 1] Control
  (:Pressed
    (CallFunction|ConsumableRequested)))

(event Input|KeyboardEvents|NumPadThree
  (params (Key :type Key%20Structure :default "None"))
  ;[1 1 1] Control
)

(event Input|KeyboardEvents|NumPadTwo
  (params (Key :type Key%20Structure :default "None"))
  ;[1 1 1] Control
)

(event Input|KeyboardEvents|NumPadOne
  (params (Key :type Key%20Structure :default "None"))
  ;[1 1 1] Control
)

(event Input|KeyboardEvents|H
  (params (Key :type Key%20Structure :default "None"))
  ;[1 1 1] Control
)

(event Input|KeyboardEvents|EAccentAigu
  (params (Key :type Key%20Structure :default "None"))
  ;[1 1 1] Control
  (:Pressed
    (CallFunction|AbilityRequested 1)))

(event Input|KeyboardEvents|Apostrophe
  (params (Key :type Key%20Structure :default "None"))
  ;[1 1 1] Control
  (:Pressed
    (CallFunction|AbilityRequested 2)))

(event Input|KeyboardEvents|Asterix
  (params (Key :type Key%20Structure :default "None"))
  ;[1 1 1] Control
  (:Pressed
    (CallFunction|AbilityRequested 3)))

(event Input|KeyboardEvents|Tilde
  (params (Key :type Key%20Structure :default "None"))
  ;[1 1 1] Control
  (:Pressed
    (CallFunction|AbilityRequested 3)))

(event Input|KeyboardEvents|LeftParantheses
  (params (Key :type Key%20Structure :default "None"))
  ;[1 1 1] Control
  (:Pressed
    (CallFunction|AbilityRequested 2)))

(event Input|KeyboardEvents|2
  (params (Key :type Key%20Structure :default "None"))
  ;[1 1 1] Control
)

(event Input|KeyboardEvents|Ù
  (params (Key :type Key%20Structure :default "None"))
  ;[1 1 1] Control
  (:Pressed
    (CallFunction|AbilityRequested 2)))

(event Input|KeyboardEvents|3
  (params (Key :type Key%20Structure :default "None"))
  ;[1 1 1] Control
)

(event Input|KeyboardEvents|G
  (params (Key :type Key%20Structure :default "None"))
  ;[1 1 1] Control
  (:Pressed
    (CallFunction|Equip5HealthPotionsforFree)))

(event Input|MouseEvents|MouseWheelDown
  (params (Key :type Key%20Structure :default "None"))
  ;[1 1 1] Control
  (:Pressed
    (if (Variables|Default|GetCanMouseRoll)
      (Variables|Default|SetCanMouseRoll false)
      (CallFunction|ConsumableDown)
      (Utilities|FlowControl|Delay 0.05)
      (Variables|Default|SetCanMouseRoll true))))

(event Input|MouseEvents|MouseWheelUp
  (params (Key :type Key%20Structure :default "None"))
  ;[1 1 1] Control
  (:Pressed
    (if (Variables|Default|GetCanMouseRoll)
      (Variables|Default|SetCanMouseRoll false)
      (CallFunction|ConsumableUp)
      (Utilities|FlowControl|Delay 0.05)
      (Variables|Default|SetCanMouseRoll true))))

(event Input|KeyboardEvents|4
  (params (Key :type Key%20Structure :default "None"))
  ;[1 1 1] Control
)

(event Input|KeyboardEvents|NumPadFour
  (params (Key :type Key%20Structure :default "None"))
  ;[1 1 1] Control
)

(event Input|KeyboardEvents|Ampersand
  (params (Key :type Key%20Structure :default "None"))
  ;[1 1 1] Control
  (:Pressed
    (CallFunction|AbilityRequested)))

(fn ConstructionScript)

(fn EquipConsumable
  (params (ConsumableIndex :type Integer) (NewConsumable :type BP%20Consumable%20Object%20Reference))
  (bind _consumablereference (Variables|Default|GetConsumableReference))
  (Utilities|Array|SetArrayElem (Variables|Default|GetEquippedConsumables) ConsumableIndex NewConsumable)
  (Default|SetEquippedasConsumable NewConsumable true)
  (bind _getroundicon (Default|GetRoundIcon NewConsumable))
  (bind _value (Default|IsMock NewConsumable))
  (if _value
    (LocalVariables|SetNewOpacity 0.0)
    (else
      (LocalVariables|SetNewOpacity 1.0)))
  (Default|ChangeConsumablePicture _consumablereference ConsumableIndex _getroundicon (LocalVariables|GetNewOpacity))
  (CallFunction|SetConsumableReady ConsumableIndex true)
  (bind _value_2 (Default|GetCooldown NewConsumable))
  (Default|SetCooldown _consumablereference ConsumableIndex _value_2))

(fn CleanConsumableSlots
  (for (_ _array_index) (Variables|Default|GetEquippedConsumables)
    (CallFunction|EquipConsumable _array_index (Variables|Default|GetMockConsumableReference))))

(fn SetClass
  (bind _self self)
  (Utilities|Casting|CastToGreystonePlayerCharacter _self
    (:then
      (Variables|Default|SetClasse "NewEnumerator0"))
    (:CastFailed
      (Utilities|Casting|CastToGideonPlayerCharacter _self
        (:then
          (Variables|Default|SetClasse "NewEnumerator1"))
        (:CastFailed
          _))
      (Utilities|Casting|CastToSparrowPlayerCharacter _self)
      (Variables|Default|SetClasse "NewEnumerator2"))))

(fn CleanConsumableSlot
  (params (Index :type Integer))
  (CallFunction|EquipConsumable Index (Variables|Default|GetMockConsumableReference)))

(fn SetConsumableReady
  (params (Index :type Integer) (Value :type Boolean))
  (Utilities|Array|SetArrayElem (Variables|Default|GetConsumableReady) Index Value))

(fn GetConsumableReady
  (params (Index :type Integer))
  (return (Utilities|Array|Get(acopy) (Variables|Default|GetConsumableReady) Index)))

(fn GetConsumableCounter
  (params (Index :type Integer))
  (return (Utilities|Array|Get(acopy) (Variables|Default|GetConsumableCounter) Index)))

(fn SetConsumableCounter
  (params (Index :type Integer) (Counter :type Float%20%28single-precision%29))
  (Utilities|Array|SetArrayElem (Variables|Default|GetConsumableCounter) Index Counter))

(fn Equip5HealthPotionsforFree
  (bind _value (Default|IsMock (Utilities|Array|Get(acopy) (Variables|Default|GetEquippedConsumables) (Variables|Default|GetSelectedConsumableIndex))))
  (if _value
    (bind _returnvalue (Game|AddComponentbyClass "/Game/Hunt/Items/BP_Consumable.BP_Consumable_C"))
    (Default|CreateHealthPotion _returnvalue (Variables|Default|GetLevel) 5)
    (CallFunction|EquipConsumable (Variables|Default|GetSelectedConsumableIndex) _returnvalue)))

(fn HealFixedValue
  (params (MoreLife :type Float%20%28single-precision%29))
  (bind _value (CallFunction|GetHealth))
  (bind _value_2 (CallFunction|GetMaxHealth))
  (if (== _value _value_2)
    (LocalVariables|SetHealedWithSuccess false)
    (elif (< (+ _value MoreLife) _value_2)
      (CallFunction|SetHealth (+ _value MoreLife))
      (LocalVariables|SetHealedWithSuccess true)
      (else
        (CallFunction|SetHealth _value_2)
        (LocalVariables|SetHealedWithSuccess true))))
  (return (LocalVariables|GetHealedWithSuccess)))

(fn GetConsumableName
  (params (Index :type Integer))
  (bind _value (Default|GetName (Utilities|Array|Get(acopy) (Variables|Default|GetEquippedConsumables) Index)))
  (return _value))

(fn SetAbilityReady
  (params (Index :type Integer) (Value :type Boolean))
  (Utilities|Array|SetArrayElem (Variables|Default|GetAbilityReady) Index Value))

(fn GetAbilityReady
  (params (Index :type Integer))
  (return (Utilities|Array|Get(acopy) (Variables|Default|GetAbilityReady) Index)))

(fn GetAbilityCounter
  (params (Index :type Integer))
  (return (Utilities|Array|Get(acopy) (Variables|Default|GetAbilityCounter) Index)))

(fn SetAbilityCounter
  (params (Index :type Integer) (Counter :type Float%20%28single-precision%29))
  (Utilities|Array|SetArrayElem (Variables|Default|GetAbilityCounter) Index Counter))

(fn EquipAbility
  (params (SpellIndex :type Integer) (NewSpell :type BP%20Spell%20Object%20Reference))
  (bind _abilitybarreference (Variables|Default|GetAbilityBarReference))
  (Utilities|Array|SetArrayElem (Variables|Default|GetEquippedAbilities) SpellIndex NewSpell)
  (bind _getroundicon (Default|GetRoundIcon NewSpell))
  (bind _value (Default|IsMock NewSpell))
  (if _value
    (Default|RemoveAbilityPicture _abilitybarreference SpellIndex)
    (else
      (Default|ChangeAbilityPicture _abilitybarreference SpellIndex _getroundicon)))
  (CallFunction|SetAbilityReady SpellIndex true)
  (bind _value_2 (Default|GetCooldown NewSpell))
  (Default|SetCooldown _abilitybarreference SpellIndex _value_2))

(fn CleanAbilitySlots
  (for (_ _array_index) (Variables|Default|GetEquippedAbilities)
    (CallFunction|EquipAbility _array_index (Variables|Default|GetMockSpellReference))))

(fn SetHeroeinDirectionOfController
  (bind _returnvalue (Pawn|GetController))
  (bind _returnvalue_2 (Pawn|GetControlRotation _returnvalue :!class /Script/Engine.Controller))
  (bind (_roll _pitch _yaw) (Math|Rotator|BreakRotator _returnvalue_2))
  (Transformation|SetActorRotation self (Math|Rotator|MakeRotator _roll 0.0 _yaw)))

(fn AddSpellsonPossessed
  (params (InputClass :type Classes%20Enum :default "NewEnumerator0"))
  (switch Utilities|FlowControl|Switch|SwitchonClasses InputClass
    (:NewEnumerator0
      (bind _returnvalue (Game|AddComponentbyClass "/Game/Hunt/Spells/Warrior/Rush.Rush_C"))
      (CallFunction|EquipAbility 0 _returnvalue)
      (bind _returnvalue_2 (Game|AddComponentbyClass "/Game/Hunt/Spells/Warrior/Tourbillon.Tourbillon_C"))
      (CallFunction|EquipAbility 1 _returnvalue_2)
      (bind _returnvalue_3 (Game|AddComponentbyClass "/Game/Hunt/Spells/Warrior/StrongAttack.StrongAttack_C"))
      (CallFunction|EquipAbility 2 _returnvalue_3)
      (bind _returnvalue_4 (Game|AddComponentbyClass "/Game/Hunt/Spells/Warrior/ShieldBoost.ShieldBoost_C"))
      (CallFunction|EquipAbility 3 _returnvalue_4))
    (:NewEnumerator1
      (bind _returnvalue_5 (Game|AddComponentbyClass "/Game/Hunt/Spells/Mage/Invocation.Invocation_C"))
      (CallFunction|EquipAbility 0 _returnvalue_5)
      (bind _returnvalue_6 (Game|AddComponentbyClass "/Game/Hunt/Spells/Mage/Tornado.Tornado_C"))
      (CallFunction|EquipAbility 1 _returnvalue_6)
      (bind _returnvalue_7 (Game|AddComponentbyClass "/Game/Hunt/Spells/Mage/Wall.Wall_C"))
      (CallFunction|EquipAbility 2 _returnvalue_7)
      (bind _returnvalue_8 (Game|AddComponentbyClass "/Game/Hunt/Spells/Mage/Ball.Ball_C"))
      (CallFunction|EquipAbility 3 _returnvalue_8))
    (:NewEnumerator2
      (bind _returnvalue_9 (Game|AddComponentbyClass "/Game/Hunt/Spells/Hunter/Invisibility.Invisibility_C"))
      (CallFunction|EquipAbility 0 _returnvalue_9)
      (bind _returnvalue_10 (Game|AddComponentbyClass "/Game/Hunt/Spells/Hunter/Multishot.Multishot_C"))
      (CallFunction|EquipAbility 1 _returnvalue_10)
      (bind _returnvalue_11 (Game|AddComponentbyClass "/Game/Hunt/Spells/Hunter/EagleJump.EagleJump_C"))
      (CallFunction|EquipAbility 2 _returnvalue_11)
      (bind _returnvalue_12 (Game|AddComponentbyClass "/Game/Hunt/Spells/Hunter/BigShot.BigShot_C"))
      (CallFunction|EquipAbility 3 _returnvalue_12))))

(fn AddSpells)