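; Player controller Blueprint for heroes that handles spawning and possessing the player's character.
; On BeginPlay it passes itself to HuntGameInstance's SpawnCharacter.
; Its two spawn events create a pawn of a given class and transform, adjusting for collision but always spawning, then call SetClass and possess it.
; The copy variant accepts a former character but never uses it, so both events behave identically.
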(event Custom|SpawnCharacter
  (params (ClassToSpawn :type BP%20Heroe%20Class%20Reference) (SpawnTransform :type Transform))
  (bind _returnvalue (Game|SpawnActorfromClass ClassToSpawn SpawnTransform "AdjustIfPossibleButAlwaysSpawn" 0 0))
  (Default|SetClass _returnvalue)
  (Pawn|Possess _returnvalue))

(event Custom|SpawnCharacterWithCopy
  (params (ClassToSpawn :type BP%20Heroe%20Class%20Reference) (SpawnTransform :type Transform) (FormerCharacter :type BP%20Heroe%20Object%20Reference))
  (bind _returnvalue (Game|SpawnActorfromClass ClassToSpawn SpawnTransform "AdjustIfPossibleButAlwaysSpawn" 0 0))
  (Default|SetClass _returnvalue)
  (Pawn|Possess _returnvalue))

(event EventBeginPlay
  (bind _ashunt_game_instance (Utilities|Casting|CastToHuntGameInstance (Game|GetGameInstance)))
  (Default|SpawnCharacter _ashunt_game_instance self))

(fn ConstructionScript)