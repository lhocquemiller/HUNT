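; BP_Servitor is the base data and registration layer for a servitor companion in Gideon's hero kit.
; On construction it registers itself with its owning BP_Character through AddServitor and stores the returned index.
; It holds a master reference and master-in-combat flag, and exposes jump, attack and forgiveness ranges through getters.
; The event graph has no active logic, so behavior using these values lives outside this Blueprint.
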(event EventBeginPlay)

(event Collision|EventActorBeginOverlap
  (params (OtherActor :type Actor%20Object%20Reference)))

(event EventTick
  (params (DeltaSeconds :type Float%20%28single-precision%29)))

(fn ConstructionScript
  (bind _asbp_character (Utilities|Casting|CastToBP_Character (Components|GetOwner)))
  (bind _servitorindex (Default|AddServitor _asbp_character self))
  (Variables|Default|SetIndexOfServitor _servitorindex))

(fn SetMaster
  (params (NewMaster :type BP%20Character%20Object%20Reference))
  (Variables|Default|SetMaster NewMaster))

(fn GetJumpRange
  (return (Variables|Default|GetJumpRange)))

(fn GetAttackRange
  (return (Variables|Default|GetAttackRange)))

(fn GetForgivenessRange
  (return (Variables|Default|GetForgivenessRange)))

(fn SetMasterinCombat
  (params (MasterInCombat :type Boolean))
  (Variables|Default|SetMasterInCombat MasterInCombat))

(fn GetMasterinCombat
  (return (Variables|Default|GetMasterInCombat)))