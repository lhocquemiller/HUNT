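; BP_Spell is a base class for hero spells, with stub ActivateSpell, RunSpell and EndSpell functions for subclasses to override.
; OnSpellActivation checks the hero's ability readiness and the Mock flag, calls SpellOnMulticast, then starts that ability's cooldown on success.
; A successful activation makes Tick call RunSpell until SpellDuration elapses, then EndSpell.
; EndOfCooldown marks the ability ready again.
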(event Custom|SpellOnMulticast
  (params (Heroe :type BP%20Heroe%20Object%20Reference))
  (bind _success (CallFunction|ActivateSpell Heroe))
  (bind _output_get (Variables|Default|SetSuccess _success))
  (if _output_get
    (Variables|Default|SetSpellIsRunning true)
    (Variables|Default|SetSpellCounter 0.0)
    (Variables|Default|SetHeroe Heroe)))

(event Custom|SpellOnServerAndMulticast
  (params (Heroe :type BP%20Heroe%20Object%20Reference))
  (CallFunction|SpellonMulticast Heroe)
  (bind _success (CallFunction|ActivateSpell Heroe))
  (bind _output_get (Variables|Default|SetSuccess _success))
  (if _output_get
    (Variables|Default|SetSpellIsRunning true)
    (Variables|Default|SetSpellCounter 0.0)
    (Variables|Default|SetHeroe Heroe)))

(event EventBeginPlay
  (CallFunction|SetRoundIcon "/Game/Hunt/Items/Icons/Empty80pixelSquareIcon.Empty80pixelSquareIcon"))

(event EventTick
  (params (DeltaSeconds :type Float%20%28single-precision%29))
  (if (Variables|Default|GetSpellIsRunning)
    (Variables|Default|SetSpellCounter (+ (Variables|Default|GetSpellCounter) DeltaSeconds))
    (CallFunction|RunSpell (Variables|Default|GetHeroe) DeltaSeconds)
    (if (>= (Variables|Default|GetSpellCounter) (Variables|Default|GetSpellDuration))
      (Variables|Default|SetSpellIsRunning false)
      (CallFunction|EndSpell (Variables|Default|GetHeroe)))))

(fn GetCooldown
  (return (Variables|Default|GetCooldown)))

(fn SetMock
  (params (Value :type Boolean))
  (bind _output_get (Variables|Default|SetMock Value))
  (if _output_get
    _))

(fn IsMock
  (return (Variables|Default|GetMock)))

(fn GetRoundIcon
  (return (Variables|Default|GetRoundIcon)))

(fn SetRoundIcon
  (params (Texture :type Texture%202D%20Object%20Reference))
  (Variables|Default|SetRoundIcon Texture))

(fn SetCooldown
  (params (NewCooldown :type Float%20%28single-precision%29))
  (Variables|Default|SetCooldown NewCooldown))

(fn ActivateSpell
  (params (Hero :type BP%20Heroe%20Object%20Reference))
  (return false))

(fn SetEffect
  (params (NewValue :type ConsumableEffect%20Enum :default "NewEnumerator0"))
  (Variables|Default|SetEffect NewValue))

(fn SetStrength
  (params (NewValue :type Float%20%28single-precision%29))
  (Variables|Default|SetStrength NewValue))

(fn OnSpellActivation
  (params (Hero :type BP%20Heroe%20Object%20Reference) (AbilityIndex :type Integer))
  (bind _output_get (Variables|Default|SetSpellIndex AbilityIndex))
  (bind _output_get_2 (LocalVariables|SetUserRef Hero))
  (bind _value (Default|GetAbilityReady _output_get_2 _output_get))
  (if _value
    (bind _value_2 (CallFunction|IsMock self))
    (if _value_2
      (Variables|Default|SetSuccess false :!label _label)
      (else
        (CallFunction|SpellonMulticast (LocalVariables|GetUserRef))
        (if (Variables|Default|GetSuccess)
          (Default|SetAbilityReady (LocalVariables|GetUserRef) (Variables|Default|GetSpellIndex) false)
          (bind _value_3 (CallFunction|GetCooldown self))
          (Default|SetAbilityCounter (LocalVariables|GetUserRef) (Variables|Default|GetSpellIndex) _value_3))))
    (else
      (goto _label)))
  (return (Variables|Default|GetSuccess)))

(fn EndOfCooldown
  (params (Hero :type BP%20Heroe%20Object%20Reference))
  (Default|SetAbilityReady Hero (Variables|Default|GetSpellIndex) true))

(fn EndSpell
  (params (Heroe :type BP%20Heroe%20Object%20Reference)))

(fn SetSpellDuration
  (params (Value :type Float%20%28single-precision%29))
  (Variables|Default|SetSpellDuration Value))

(fn GetSpellDuration
  (return (Variables|Default|GetSpellDuration)))

(fn RunSpell
  (params (Hero :type BP%20Heroe%20Object%20Reference) (TimeDiff :type Float%20%28single-precision%29)))