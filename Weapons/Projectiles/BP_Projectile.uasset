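; BP_Projectile is a weapon projectile actor that destroys itself after TimeUntilDisappear.
; When its Mesh ends an overlap with an actor other than its owner, it applies Damages once, guarded by HitOnce, then destroys itself.
; Damage triggers on overlap end rather than begin, and any blocking hit on the Mesh zeroes Damages without destroying the projectile.
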(event OnComponentHit(Mesh)
  (params (HitComponent :type Primitive%20Component%20Object%20Reference) (OtherActor :type Actor%20Object%20Reference) (OtherComp :type Primitive%20Component%20Object%20Reference) (NormalImpulse :type Vector :default "0, 0, 0") (Hit :type Hit%20Result%20Structure%20%28by%20ref%29))
  (Variables|Default|SetDamages 0.0))

(event OnComponentEndOverlap(Mesh)
  (params (OverlappedComponent :type Primitive%20Component%20Object%20Reference) (OtherActor :type Actor%20Object%20Reference) (OtherComp :type Primitive%20Component%20Object%20Reference) (OtherBodyIndex :type Integer))
  (bind _returnvalue (Components|GetOwner))
  (if (!= OtherActor _returnvalue)
    (if (not (Variables|Default|GetHitOnce))
      (Game|Damage|ApplyDamage OtherActor (Variables|Default|GetDamages) 0 _returnvalue)
      (Variables|Default|SetHitOnce true)
      (Actor|DestroyActor self))))

(event EventBeginPlay
  (Utilities|FlowControl|Delay (Variables|Default|GetTimeUntilDisappear))
  (Actor|DestroyActor))

(fn ConstructionScript)